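; Turret enemy that tracks and shoots at the player's copter while it is inside a detection sphere.
; Overlap starts a timeline whose updates yaw the main body, pitch the launcher within a clamped range and aim both muzzles at the target.
; A Delay inside the update throttles fire, spawning bullets from a random muzzle unless the player is dead.
; Any damage decrements Hp, and a hit at zero destroys the turret.
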(event `self.Sphere.OnComponentBeginOverlap`
  (params (OverlappedComponent :type "PrimitiveComponent Object Reference") (OtherActor :type "Actor Object Reference") (OtherComp :type "PrimitiveComponent Object Reference") (OtherBodyIndex :type Integer) (bFromSweep :type Boolean) (SweepResult :type "HitResult Structure (by ref)"))
  (bind _returnvalue (`self.K2_GetActorLocation` OtherActor))
  (bind _bul (`self.bul`))
  (bind _roll (.roll (`self.K2_GetActorRotation` self)))
  (if (`self.ActorHasTag` OtherActor "player")
    (bind _ascopter (cast `/Game/blueprints/copter` OtherActor))
    (set `self.player` _ascopter)
    (`Timeline|Timeline` :`NewTime` 0.1 :!via `PlayFromStart` :!label _label
      (:`Update`
        (`SceneComponent.K2_SetWorldRotation` (`self.muzzle_1`) (`KismetMathLibrary.FindLookAtRotation` (`SceneComponent.K2_GetComponentLocation` (`self.muzzle_1`)) _returnvalue) false false)
        (`SceneComponent.K2_SetWorldRotation` (`self.muzzle_2`) (`KismetMathLibrary.FindLookAtRotation` (`SceneComponent.K2_GetComponentLocation` (`self.muzzle_2`)) _returnvalue) false false)
        (`SceneComponent.K2_SetRelativeRotation` (`self.main`) (`KismetMathLibrary.MakeRotator` _roll (.pitch (`self.K2_GetActorRotation` self)) (.yaw (`KismetMathLibrary.FindLookAtRotation` (`self.K2_GetActorLocation` self) _returnvalue))) false false)
        (`SceneComponent.K2_SetRelativeRotation` (`self.launcher`) (`KismetMathLibrary.MakeRotator` _roll (`KismetMathLibrary.FClamp` (.pitch (`KismetMathLibrary.FindLookAtRotation` (`self.K2_GetActorLocation` self) _returnvalue)) 0.0 30.0) (.yaw (`self.K2_GetActorRotation` self))) false false)
        (`KismetSystemLibrary.Delay` 0.7)
        (if (`/Game/blueprints/copter.dead` (`self.player`))
          _
          (elif (`KismetMathLibrary.RandomBool`)
            (`|SpawnActorFromClass` _bul (`SceneComponent.K2_GetComponentToWorld` (`self.muzzle_1`)) "AlwaysSpawn" "MultiplyWithRoot" null null)
            (else
              (`|SpawnActorFromClass` _bul (`SceneComponent.K2_GetComponentToWorld` (`self.muzzle_2`)) "AlwaysSpawn" "MultiplyWithRoot" null null))))))))

(event `self.Sphere.OnComponentEndOverlap`
  (params (OverlappedComponent :type "PrimitiveComponent Object Reference") (OtherActor :type "Actor Object Reference") (OtherComp :type "PrimitiveComponent Object Reference") (OtherBodyIndex :type Integer))
  (if (`self.ActorHasTag` OtherActor "player")
    (goto _label :!via `Stop`)))

(event `self.ReceiveAnyDamage`
  (params (Damage :type "Float (single-precision)") (DamageType :type "DamageType Object Reference") (InstigatedBy :type "Controller Object Reference") (DamageCauser :type "Actor Object Reference"))
  (`self.damage`))

(fn `damage`
  (if (> (`self.hp`) 0)
    (bind _result (`/Engine/EditorBlueprintResources/StandardMacros.DecrementInt` (`self.hp`))
      (:`  `
        (set `self.hp` _result)))
    (else
      (`self.K2_DestroyActor`))))

(fn `UserConstructionScript`)