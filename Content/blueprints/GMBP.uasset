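; GMBP, apparently a game mode, manages the player's HUD for a game with a Copter as the player.
; On BeginPlay it creates the Hud widget, adds it to the viewport, stores the Copter found in the level as Player and sets that Copter's Gm to None.
; UpdateHp and UpdateAmmo push the Player's current health and ammo into the HUD, with Tick left unused.
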(event `self.ReceiveBeginPlay`
  (bind _returnvalue (`|GenericCreateObject` "/Game/blueprints/hud.hud_C"))
  (set `self.hud` _returnvalue)
  (`UserWidget.AddToViewport` _returnvalue 0)
  (bind _returnvalue_2 (`GameplayStatics.GetActorOfClass` "/Game/blueprints/copter.copter_C"))
  (set `self.player` _returnvalue_2)
  (set `/Game/blueprints/copter.gm` null self _returnvalue_2))

(fn `update_ammo`
  (`/Game/blueprints/hud.update_ammo` (`self.hud`) (`/Game/blueprints/copter.ammo` (`self.player`))))

(fn `update_hp`
  (`/Game/blueprints/hud.update_bar` (`self.hud`) (`/Game/blueprints/copter.hp` (`self.player`))))

(fn `UserConstructionScript`)