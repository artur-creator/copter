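; Player-controlled copter pawn that flies, shoots and tracks its own health and ammo.
; Axis inputs drive look and movement along its forward, right and up vectors, and shooting spends ammo to spawn Bul at the Muzzle.
; Damage lowers Hp, and a hit taken with none left sets Dead and restarts via Gm.
; Heal and Recharge refill up to a cap, with Gm notified of Hp and ammo changes.
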(event `InputAxis|look_right`
  (params (AxisValue :type "Float (single-precision)"))
  (`self.AddControllerYawInput` AxisValue))

(event `InputAxis|look_up`
  (params (AxisValue :type "Float (single-precision)"))
  (`self.AddControllerPitchInput` (* AxisValue -1.0)))

(event `InputAxis|forward`
  (params (AxisValue :type "Float (single-precision)"))
  (`self.AddMovementInput` (`self.GetActorForwardVector`) AxisValue))

(event `InputAxis|right`
  (params (AxisValue :type "Float (single-precision)"))
  (`self.AddMovementInput` (`self.GetActorRightVector`) AxisValue))

(event `InputAxis|fly`
  (params (AxisValue :type "Float (single-precision)"))
  (`self.AddMovementInput` (`self.GetActorUpVector`) AxisValue))

(event `InputAction|shot`
  (params (Key :type "Key Structure"))
  (:`Pressed`
    (if (> (`self.ammo`) 0)
      (bind _result (`/Engine/EditorBlueprintResources/StandardMacros.DecrementInt` (`self.ammo`))
        (:`  `
          (set `self.ammo` _result)
          (`|SpawnActorFromClass` (`self.bul`) (`SceneComponent.K2_GetComponentToWorld` (`self.muzzle`)) "AlwaysSpawn" "MultiplyWithRoot" null null)
          (`/Game/blueprints/master.update_ammo` (`self.gm`)))))))

(event `self.ReceiveAnyDamage`
  (params (Damage :type "Float (single-precision)") (DamageType :type "DamageType Object Reference") (InstigatedBy :type "Controller Object Reference") (DamageCauser :type "Actor Object Reference"))
  (if (> (`self.hp`) 0.0)
    (set `self.hp` (- (`self.hp`) Damage))
    (`/Game/blueprints/master.update_hp` (`self.gm`))
    (else
      (set `self.dead` true)
      (`GameMode.RestartGame` (`self.gm`)))))

(fn `heal`
  (params (amount :type "Float (double-precision)"))
  (bind _returnvalue (+ amount (`self.hp`)))
  (if (> _returnvalue 100.0)
    (set `self.hp` 100.0)
    (else
      (set `self.hp` _returnvalue)))
  (`/Game/blueprints/master.update_hp` (`self.gm`)))

(fn `recharge`
  (params (amount :type Integer))
  (bind _returnvalue (+ amount (`self.ammo`)))
  (if (> _returnvalue 100)
    (set `self.ammo` 100)
    (else
      (set `self.ammo` _returnvalue)))
  (`/Game/blueprints/master.update_ammo` (`self.gm`)))

(fn `UserConstructionScript`)